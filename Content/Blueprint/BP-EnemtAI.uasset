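; Enemy character Blueprint that chases the player and knocks them back with a melee attack.
; PawnSensing sighting of any pawn triggers ChasePlayer, which runs AI MoveTo toward player 0.
; On arrival it plays an attack montage, with CanAttack blocking repeat attacks until the montage completes or is interrupted.
; A montage notify fires a forward sphere trace with debug drawing, launching any hit Character forward and upward.
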(event OnSeePawn(PawnSensing)
  (params (Pawn :type Pawn%20Object%20Reference))
  ;[0.15 0.15 0.15 0.5] 看见玩家检查
  (CallFunction|ChasePlayer))

(event Custom|Chase%20Player
  (bind _returnvalue (Transformation|GetActorLocation))
  ;[0.15 0.15 0.15 0.5] 追主角
  (AI|AIMoveTo self "0, 0, 0" (Game|GetPlayerCharacter 0) 1.2e+02 false
    (:OnSuccess
      ;[0.15 0.15 0.15 0.5] 攻击
      (if (Variables|Default|GetcanAttack)
        (Animation|Montage|PlayMontage (Variables|Character|GetMesh) "/Game/Characters/Villager/animation/Attack/A_Attack_Montage.A_Attack_Montage"
          (:then
            (Variables|Default|SetcanAttack false))
          (:OnCompleted
            (Variables|Default|SetcanAttack true :!label _label))
          (:OnInterrupted
            (goto _label))
          (:OnNotifyBegin
            ;[0.15 0.15 0.15 0.5] 受击检测
            (bind (_outhit _returnvalue_2) (Collision|SphereTraceByChannel _returnvalue (+ _returnvalue (* (Math|Vector|GetForwardVector (Transformation|GetActorRotation)) 1.8e+02)) 25.0 "TraceTypeQuery3" false 0 "ForDuration" true "(R=1.000000,G=0.000000,B=0.000000,A=1.000000)" "(R=0.000000,G=1.000000,B=0.000000,A=1.000000)" 0.5))
            (if _returnvalue_2
              ;[0.15 0.15 0.15 0.5] 击飞
              (bind _as角色 (Utilities|Casting|CastToCharacter (.HitActor (Collision|BreakHitResult _outhit))))
              (Character|LaunchCharacter _as角色 (+ (* (Math|Vector|GetForwardVector (Transformation|GetActorRotation)) (Variables|Default|GetFrontal%20Knockbar)) (Math|Vector|MakeVector 0.0 0.0 (Variables|Default|GetupwardsKnockback))) false false))))))))

(fn ConstructionScript)