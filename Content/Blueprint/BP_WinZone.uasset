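; BP_WinZone is a goal trigger that ends the game when an actor tagged "Ball" overlaps its DetectArea component.
; On overlap it shows the WPB_GameOver widget, enables the mouse cursor, switches to UI-only input and pauses the game.
; It then removes the persistent HUD through the HUDRef held by the player's BP_ThirdPersonCharacter.
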(event OnComponentBeginOverlap(DetectArea)
  (params (OverlappedComponent :type Primitive%20Component%20Object%20Reference) (OtherActor :type Actor%20Object%20Reference) (OtherComp :type Primitive%20Component%20Object%20Reference) (OtherBodyIndex :type Integer) (bFromSweep :type Boolean) (SweepResult :type Hit%20Result%20Structure%20%28by%20ref%29))
  (bind _returnvalue (Game|GetPlayerController 0))
  (if (Actor|ActorHasTag OtherActor "Ball")
    (bind _returnvalue_2 (UserInterface|CreateWidget "/Game/UI/WPB_GameOver.WPB_GameOver_C" _returnvalue))
    (UserInterface|Viewport|AddtoViewport _returnvalue_2 0)
    (Variables|/Script/Engine.PlayerController|SetbShowMouseCursor _returnvalue true)
    (Input|SetInputModeUIOnly _returnvalue _returnvalue_2 "DoNotLock" false)
    (Game|SetGamePaused true)
    ;[0.15 0.15 0.15 0.5] 销毁常驻UI
    (bind _asbp_third_person_character (Utilities|Casting|CastToBP_ThirdPersonCharacter (Game|GetPlayerCharacter 0)))
    (Widget|RemovefromParent (Variables|/Game/Blueprint/BP_ThirdPersonCharacter.BP_ThirdPersonCharacter_C|GetHUD_Ref _asbp_third_person_character))))

(event EventBeginPlay)

(event Collision|EventActorBeginOverlap
  (params (OtherActor :type Actor%20Object%20Reference)))

(event EventTick
  (params (DeltaSeconds :type Float%20%28single-precision%29)))

(fn ConstructionScript)